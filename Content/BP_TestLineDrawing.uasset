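; BP_TestLineDrawing is a test Blueprint that exercises a LineMesh component's create, update and remove calls through keyboard input.
; GeneratePoints fills a shared Points array with random positions in a box, offset by Centroid, which F sets to zero through an empty random range.
; F adds a green 100-point line section, G rewrites a randomly chosen section with 200 red points, and H removes all lines.
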(event `self.ReceiveBeginPlay`)

(event `Key|F`
  (params (Key :type "Key Structure"))
  (:`Pressed`
    (set `self.Centroid` (`KismetMathLibrary.RandomFloatInRange` 0.0))
    (`self.GeneratePoints` 100
      (:`Completed`
        (`LineMeshComponent.CreateLine` (`self.LineMesh`) (`LineMeshComponent.GetNumLines` (`self.LineMesh`)) (`self.Points`) (make `LinearColor` 0.0 128.0 0.0 128.0))))))

(event `Key|G`
  (params (Key :type "Key Structure"))
  (:`Pressed`
    (`self.GeneratePoints` 200
      (:`Completed`
        (`LineMeshComponent.UpdateLine` (`self.LineMesh`) (`KismetMathLibrary.RandomIntegerInRange` 0 (- (`LineMeshComponent.GetNumLines` (`self.LineMesh`)) 1)) (`self.Points`) (make `LinearColor` 255.0 0.0 0.0 255.0))))))

(event `Key|H`
  (params (Key :type "Key Structure"))
  (:`Pressed`
    (`LineMeshComponent.RemoveAllLines` (`self.LineMesh`))))

(fn `UserConstructionScript`)