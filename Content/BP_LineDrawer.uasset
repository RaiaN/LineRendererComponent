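; Line drawer Blueprint that exercises a LineRenderer component through number-key input, apparently as a test or demo.
; Keys create or update two-point lines in two indexed sections, with endpoints from GetRandomPoint, preset colors, and random thickness on updates.
; Other keys toggle each section's visibility through FlipFlops, remove either line by index, or clear all lines.
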(event `Key|One`
  (params (Key :type "Key Structure"))
  (:`Pressed`
    (`LineRendererComponent.CreateLine` (`self.LineRenderer`) 0 (`|MakeArray` (`self.GetRandomPoint`) (`self.GetRandomPoint`)) (`KismetMathLibrary.LinearColor_Black`) 2.0)))

(event `Key|Two`
  (params (Key :type "Key Structure"))
  (:`Pressed`
    (`LineRendererComponent.CreateLine` (`self.LineRenderer`) 1 (`|MakeArray` (`self.GetRandomPoint`) (`self.GetRandomPoint`)) (`KismetMathLibrary.LinearColor_Red`) 8.0)))

(event `Key|Three`
  (params (Key :type "Key Structure"))
  (:`Pressed`
    (`LineRendererComponent.UpdateLine` (`self.LineRenderer`) 0 (`|MakeArray` (`self.GetRandomPoint`) (`self.GetRandomPoint`)) (`KismetMathLibrary.LinearColor_Green`) (`KismetMathLibrary.RandomFloatInRange` 2.0 10.0))))

(event `Key|Four`
  (params (Key :type "Key Structure"))
  (:`Pressed`
    (`LineRendererComponent.UpdateLine` (`self.LineRenderer`) 1 (`|MakeArray` (`self.GetRandomPoint`) (`self.GetRandomPoint`)) (`KismetMathLibrary.LinearColor_Green`) (`KismetMathLibrary.RandomFloatInRange` 2.0 10.0))))

(event `Key|Five`
  (params (Key :type "Key Structure"))
  (:`Pressed`
    (bind _isa (`/Engine/EditorBlueprintResources/StandardMacros.FlipFlop`)
      (:`A`
        _)
      (:`B`
        _))
    (`LineRendererComponent.SetLineVisible` (`self.LineRenderer`) 0 (not _isa))))

(event `Key|Six`
  (params (Key :type "Key Structure"))
  (:`Pressed`
    (bind _isa (`/Engine/EditorBlueprintResources/StandardMacros.FlipFlop`)
      (:`A`
        _)
      (:`B`
        _))
    (`LineRendererComponent.SetLineVisible` (`self.LineRenderer`) 1 (not _isa))))

(event `Key|Seven`
  (params (Key :type "Key Structure"))
  (:`Pressed`
    (`LineRendererComponent.RemoveLine` (`self.LineRenderer`) 0)))

(event `Key|Eight`
  (params (Key :type "Key Structure"))
  (:`Pressed`
    (`LineRendererComponent.RemoveLine` (`self.LineRenderer`) 1)))

(event `Key|Nine`
  (params (Key :type "Key Structure"))
  (:`Pressed`
    (`LineRendererComponent.RemoveAllLines` (`self.LineRenderer`))))

(fn `UserConstructionScript`)